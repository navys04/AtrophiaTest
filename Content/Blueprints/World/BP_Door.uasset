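; Interactable door actor that swings open and closed on alternating interactions.
; The Interaction component's OnInteract event drives a FlipFlop that plays separate open and close timelines from the start, each setting DoorPivot's relative yaw from its DoorRotationZ track.
; OpenDoor is an empty stub, and CloseDoor holds a single RInterpTo rotation step that the event graph never calls.
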(event OnInteract(Interaction)
  (Utilities|FlowControl|FlipFlop
    (:A
      (bind _doorrotationz (Timeline|Timeline_DoorOpen PlayFromStart)
        (:Update
          (Transformation|SetRelativeRotation (Variables|Default|GetDoorPivot) (Math|Rotator|MakeRotator 0.0 0.0 _doorrotationz) false false))))
    (:B
      (bind _doorrotationz_2 (Timeline|Timeline_DoorClose PlayFromStart)
        (:Update
          (Transformation|SetRelativeRotation (Variables|Default|GetDoorPivot) (Math|Rotator|MakeRotator 0.0 0.0 _doorrotationz_2) false false))))))

(fn ConstructionScript)

(fn OpenDoor)

(fn CloseDoor
  (bind _doorpivot (Variables|Default|GetDoorPivot))
  (Transformation|SetWorldRotation _doorpivot (Math|Interpolation|RInterpTo (Transformation|GetWorldRotation _doorpivot) "0,50.000000, 0" (Utilities|Time|GetWorldDeltaSeconds) 0.3) false false))